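; Enemy actor for Fractured Citadel with a skeletal mesh and a selection box.
; On BeginPlay it finds the BP_TopDownCharacter and rotates once to face it, using a full look-at rotation.
; Each tick, while the selection box is visible, it rescales the box to the skeletal mesh's bounds extent divided by 100.
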(event `self.ReceiveTick`
  (params (DeltaSeconds :type "Float (single-precision)"))
  (bind _selectionbox (`self.SelectionBox`))
  (if (`SceneComponent.IsVisible` _selectionbox)
    (`SceneComponent.SetWorldScale3D` _selectionbox (/ (`.BoxExtent` (`KismetSystemLibrary.GetComponentBounds` (`self.SkeletalMesh`))) 100.0))))

(event `self.ReceiveBeginPlay`
  (bind _returnvalue (`GameplayStatics.GetActorOfClass` "/Game/TopDown/Blueprints/BP_TopDownCharacter.BP_TopDownCharacter_C"))
  (`self.K2_SetActorRotation` (`KismetMathLibrary.FindLookAtRotation` (`self.K2_GetActorLocation`) (`self.K2_GetActorLocation` _returnvalue))))

(fn `UserConstructionScript`)