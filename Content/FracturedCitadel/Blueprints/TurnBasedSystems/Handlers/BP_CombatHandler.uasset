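; Actor that runs a turn-based combat encounter, using WBP_CombatHUD icons as the roster and turn order.
; StartCombat spawns the damage-number handler and sorts icon owners into player and enemy arrays.
; Tick recounts both sides and checks the first ordered icon, triggering a delay-paced enemy turn that damages a random player icon.
; When either side empties, EndCombat clears icons, blends the view to player characters, hides the HUD and destroys itself.
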(event `self.ReceiveBeginPlay`
  (bind _foundwidgets (`WidgetBlueprintLibrary.GetAllWidgetsOfClass` "/Game/FracturedCitadel/Blueprints/TurnBasedSystems/UI/WBP_CombatHUD.WBP_CombatHUD_C"))
  (for _array_element _foundwidgets
    (set `self.CombatHUD` _array_element))
  (set `self.BaseCombatCameraTransform` (`SceneComponent.K2_GetComponentToWorld` (`self.CombatCamera`)))
  (set `/Game/FracturedCitadel/Blueprints/TurnBasedSystems/UI/WBP_CombatHUD.CombatActive` true (`self.CombatHUD`)))

(event `StartCombat`
  (bind _returnvalue (`|SpawnActorFromClass` "/Game/FracturedCitadel/Blueprints/TurnBasedSystems/UI/DMGNumbers/BP_DMGNumHandler.BP_DMGNumHandler_C" (`self.GetTransform` self) "Undefined" "MultiplyWithRoot" null null))
  (bind _output_get (set `self.DMGHandler` _returnvalue))
  (set `/Game/FracturedCitadel/Blueprints/TurnBasedSystems/UI/WBP_CombatHUD.DMGHandler` _output_get (`self.CombatHUD`))
  (for _array_element (`/Game/FracturedCitadel/Blueprints/TurnBasedSystems/UI/WBP_CombatHUD.IconArray` (`self.CombatHUD`))
    (bind _isplayer (`/Game/FracturedCitadel/Blueprints/TurnBasedSystems/UI/WBP_TurnIcon.IsOwnerPlayer` _array_element))
    (if _isplayer
      (`KismetArrayLibrary.Array_Add` (`self.BPPlayerArray`) (`/Game/FracturedCitadel/Blueprints/TurnBasedSystems/UI/WBP_TurnIcon.PlayerOwner` _array_element))
      (`KismetArrayLibrary.Array_Add` (`self.PlayerIconArray`) _array_element)
      (else
        (`KismetArrayLibrary.Array_Add` (`self.BPEnemyArray`) (`/Game/FracturedCitadel/Blueprints/TurnBasedSystems/UI/WBP_TurnIcon.EnemyOwner` _array_element))
        (`KismetArrayLibrary.Array_Add` (`self.EnemyIconArray`) _array_element)))
    (bind _isplayerturn (`self.IsPlayerTurn`))
    (set `self.PlayersTurn` _isplayerturn)))

(event `self.ReceiveTick`
  (params (DeltaSeconds :type "Float (single-precision)"))
  (`self.UpdateEntityCount`)
  (if (or (<= (`self.AllyCount`) 0) (<= (`self.EnemyCount`) 0))
    (`self.End Combat`)
    (else
      (bind _isplayerturn (`self.IsPlayerTurn`))
      (if _isplayerturn
        _
        (elif (not (`self.DoingEnemyTurn`))
          (`self.DoEnemyTurn`)
          (set `self.DoingEnemyTurn` true))))))

(event `DoEnemyTurn`
  (bind _currentturnicon (`self.CurrentTurnIcon`))
  (for _array_element (`/Game/FracturedCitadel/Blueprints/TurnBasedSystems/UI/WBP_CombatHUD.OrganizedIconArray` (`self.CombatHUD`))
    (`/Game/FracturedCitadel/Blueprints/TurnBasedSystems/UI/WBP_TurnIcon.DeselectIcon` _array_element))
  (`KismetSystemLibrary.Delay` (/ 2.0 (`self.DelaySpeed`)))
  (set `/Game/FracturedCitadel/Blueprints/TurnBasedSystems/UI/WBP_TurnIcon.Hovered` true _currentturnicon)
  (`/Game/FracturedCitadel/Blueprints/TurnBasedSystems/UI/WBP_TurnIcon.ShowBox` _currentturnicon)
  (`KismetSystemLibrary.Delay` (/ 1.0 (`self.DelaySpeed`)))
  (`/Game/FracturedCitadel/Blueprints/TurnBasedSystems/UI/WBP_TurnIcon.HideBox` (`self.CurrentTurnIcon`))
  (`/Game/FracturedCitadel/Blueprints/TurnBasedSystems/UI/WBP_CombatHUD.BeginAiming` (`self.CombatHUD`))
  (`KismetSystemLibrary.Delay` (/ 1.0 (`self.DelaySpeed`)))
  (set `/Game/FracturedCitadel/Blueprints/TurnBasedSystems/UI/WBP_TurnIcon.Hovered` false (`self.CurrentTurnIcon`))
  (`/Game/FracturedCitadel/Blueprints/TurnBasedSystems/UI/WBP_TurnIcon.SelectIcon` (`KismetArrayLibrary.Array_Random` (`self.PlayerIconArray`)))
  (`KismetSystemLibrary.Delay` (/ 1.0 (`self.DelaySpeed`)))
  (`/Game/FracturedCitadel/Blueprints/TurnBasedSystems/UI/WBP_CombatHUD.DamageSelected` (`self.CombatHUD`) (`FracturedCitadelEnemy.enemyCurrentDamage` (`/Game/FracturedCitadel/Blueprints/TurnBasedSystems/UI/WBP_TurnIcon.EnemyOwner` (`self.CurrentTurnIcon`))))
  (`KismetSystemLibrary.Delay` (/ 2.0 (`self.DelaySpeed`)))
  (`/Game/FracturedCitadel/Blueprints/TurnBasedSystems/UI/WBP_CombatHUD.PlayOutTurn` (`self.CombatHUD`))
  (set `self.DoingEnemyTurn` false))

(event `End Combat`
  (bind _combathud (`self.CombatHUD`))
  (bind _combathud_2 (`self.CombatHUD`))
  (for _array_element (`/Game/FracturedCitadel/Blueprints/TurnBasedSystems/UI/WBP_CombatHUD.IconArray` _combathud)
    (bind _isplayer (`/Game/FracturedCitadel/Blueprints/TurnBasedSystems/UI/WBP_TurnIcon.IsOwnerPlayer` _array_element))
    (if _isplayer
      (`/Game/FracturedCitadel/Blueprints/TurnBasedSystems/UI/WBP_CombatHUD.KillIcon` _combathud null (`/Game/FracturedCitadel/Blueprints/TurnBasedSystems/UI/WBP_TurnIcon.PlayerOwner` _array_element) true)
      (else
        (`/Game/FracturedCitadel/Blueprints/TurnBasedSystems/UI/WBP_CombatHUD.KillIcon` _combathud (`/Game/FracturedCitadel/Blueprints/TurnBasedSystems/UI/WBP_TurnIcon.EnemyOwner` _array_element) null false))))
  (`KismetSystemLibrary.CollectGarbage`)
  (`self.K2_DestroyActor` (`self.DMGHandler`))
  (for _array_element_2 (`self.BPPlayerArray`)
    (`/Game/TopDown/Blueprints/BP_TopDownCharacter.DeactivateCameras` _array_element_2)
    (`ActorComponent.Activate` (`FracturedCitadelCharacter.CameraBoom` _array_element_2) false)
    (`ActorComponent.Activate` (`FracturedCitadelCharacter.TopDownCameraComponent` _array_element_2) false)
    (`ActorComponent.Activate` (`Character.CharacterMovement` _array_element_2) false)
    (`PlayerController.SetViewTargetWithBlend` (`GameplayStatics.GetPlayerController` 0) _array_element_2 1.5 "VTBlend_EaseInOut" 2.0 false))
  (set `/Game/FracturedCitadel/Blueprints/TurnBasedSystems/UI/WBP_CombatHUD.CombatActive` false _combathud_2)
  (`Widget.SetVisibility` _combathud_2 "Hidden")
  (`self.K2_DestroyActor`))

(fn `IsPlayerTurn`
  (returns (isPlayerTurn :type Boolean))
  (for _array_element (`/Game/FracturedCitadel/Blueprints/TurnBasedSystems/UI/WBP_CombatHUD.OrganizedIconArray` (`self.CombatHUD`))
    (bind _output_get (set `self.PlayersTurn` (`KismetSystemLibrary.IsValid` (`/Game/FracturedCitadel/Blueprints/TurnBasedSystems/UI/WBP_TurnIcon.PlayerOwner` _array_element))))
    (return _output_get)))

(fn `UpdateEntityCount`
  (set `self.EnemyCount` 0)
  (set `self.AllyCount` 0)
  (for _array_element (`/Game/FracturedCitadel/Blueprints/TurnBasedSystems/UI/WBP_CombatHUD.OrganizedIconArray` (`self.CombatHUD`))
    (bind _isplayer (`/Game/FracturedCitadel/Blueprints/TurnBasedSystems/UI/WBP_TurnIcon.IsOwnerPlayer` _array_element))
    (if _isplayer
      (`/Engine/EditorBlueprintResources/StandardMacros.IncrementInt` (`self.AllyCount`))
      (else
        (`/Engine/EditorBlueprintResources/StandardMacros.IncrementInt` (`self.EnemyCount`))))))

(fn `UserConstructionScript`)